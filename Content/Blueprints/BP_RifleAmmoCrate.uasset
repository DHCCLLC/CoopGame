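; Ammo crate pickup that adds its ammunition type and count to the inventory of an overlapping PlayerPawn.
; It tells the inventory component whether that type matches the pawn's current weapon, and destroys itself only if the add succeeds.
; A Hover timeline is set up to bob and spin the crate, but nothing in the graph triggers it.
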(event `self.ReceiveBeginPlay`)

(event `self.ReceiveActorBeginOverlap`
  (params (OtherActor :type "Actor Object Reference"))
  (bind _ammunitiontype (`self.AmmunitionType`))
  (bind _asplayer_pawn (cast `/Game/Blueprints/PlayerPawn` OtherActor))
  (bind _returnvalue (`SCharacter.GetWeaponAmmunitionType` _asplayer_pawn))
  (bind _returnvalue_2 (`SInventoryComponent.AddAmmunition` (`SCharacter.InventoryComp` _asplayer_pawn) _ammunitiontype (`self.AmmunitionCount`) (`|EnumEquality` _returnvalue _ammunitiontype)))
  (if _returnvalue_2
    (`self.K2_DestroyActor`)))

(fn `UserConstructionScript`)